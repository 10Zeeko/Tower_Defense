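; BPC_MoveToTarget is a bullet component that homes its owning actor in on a target actor.
; Each tick it moves the owner straight toward MTarget's current location at MSpeed, scaled by delta time, and rotates it to face the target.
; If MTarget is no longer valid, it destroys the owner.
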(event `self.ReceiveTick`
  (params (DeltaSeconds :type "Float (single-precision)"))
  (bind _returnvalue (`self.GetOwner`))
  (bind _returnvalue_2 (`Actor.K2_GetActorLocation` (`self.GetOwner`)))
  (bind _returnvalue_3 (`Actor.K2_GetActorLocation` (`self.mTarget`)))
  (`self.mTarget`
    (:`then`
      (`Actor.K2_SetActorLocationAndRotation` _returnvalue (+ (* (* DeltaSeconds (`self.mSpeed`)) (`KismetMathLibrary.Normal` (- _returnvalue_3 _returnvalue_2))) _returnvalue_2) (`KismetMathLibrary.FindLookAtRotation` _returnvalue_2 _returnvalue_3) false false))
    (:`else`
      (`Actor.K2_DestroyActor` _returnvalue))))