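; Tower defense tower that automatically fires projectiles at enemies entering its range.
; On BeginPlay it loads damage, bullet speed, fire rate and range from its tower info, then starts a looping timer at the inverse fire rate.
; Capsule overlaps maintain the list of enemies in range.
; Each tick picks the first living enemy, turns the AxisX pivot horizontally toward it and spawns a bullet that moves to that target.
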(event `self.ReceiveBeginPlay`
  (bind ((`Damage_11_8A74182A474E021B7C51DFA54A01F5A5` _damage) (`BulletSpeed_13_327CF2B8463FE1F348BDF98323C9D578` _bulletspeed) (`TowerFireRate_27_E511C6FF4AA2F5FE41A3FBAD7E5F1B10` _towerfirerate) (`TowerRange_18_4AC1814442E25269B5F82186697AF0BE` _towerrange)) (break `/Game/Blueprints/Weapons/sTowerInfo` (`self.mTowerInfo`)))
  (`|ExecutionSequence`
    (:`then_0`
      (set `self.mDamage` _damage)
      (set `self.mBulletSpeed` _bulletspeed)
      (set `self.mFireRate` _towerfirerate)
      (`CapsuleComponent.SetCapsuleRadius` (`self.C_CheckEnemy`) _towerrange true))
    (:`then_1`
      (bind _returnvalue (`KismetSystemLibrary.K2_SetTimerDelegate` (delegate `TowerTick`) (`self.GetFireRate` (`self.mFireRate`)) true))
      (set `self.mCurrentTimer` _returnvalue))))

(event `SetFireRate`
  (params (aFireRate :type "Float (double-precision)"))
  (bind _output_get (set `self.mFireRate` (`self.GetFireRate` aFireRate)))
  (`KismetSystemLibrary.K2_InvalidateTimerHandle` (`self.mCurrentTimer`))
  (`KismetSystemLibrary.K2_SetTimerDelegate` (delegate `TowerTick`) _output_get true))

(event `TowerTick`
  (set `self.mTarget` (`self.GetEnemyToFocus`))
  (`self.RotateToEnemy`)
  (`self.mTarget`
    (:`then`
      (bind _returnvalue (`|SpawnActorFromClass` (`self.mBulletType`) (`SceneComponent.K2_GetComponentToWorld` (`self.ShootPoint`)) "AlwaysSpawn" "MultiplyWithRoot" null (`self.mBulletSpeed`) (`self.mDamage`) null))
      (set `/Game/Blueprints/Weapons/Bullets/Components/BPC_MoveToTarget.mTarget` (`self.mTarget`) (`/Game/Blueprints/Weapons/Bullets/BP_BulletBase.BPC_MoveToTarget` _returnvalue)))
    (:`else`)))

(event `self.C_CheckEnemy.OnComponentBeginOverlap`
  (params (OverlappedComponent :type "PrimitiveComponent Object Reference") (OtherActor :type "Actor Object Reference") (OtherComp :type "PrimitiveComponent Object Reference") (OtherBodyIndex :type Integer) (bFromSweep :type Boolean) (SweepResult :type "HitResult Structure (by ref)"))
  (bind _asbp_enemy_base (cast `/Game/Blueprints/Enemies/BP_EnemyBase` OtherActor))
  (`self.CheckIndex` _asbp_enemy_base
    (:`then`
      (`KismetArrayLibrary.Array_Add` (`self.mEnemiesInRange`) _asbp_enemy_base))))

(event `self.C_CheckEnemy.OnComponentEndOverlap`
  (params (OverlappedComponent :type "PrimitiveComponent Object Reference") (OtherActor :type "Actor Object Reference") (OtherComp :type "PrimitiveComponent Object Reference") (OtherBodyIndex :type Integer))
  (bind _asbp_enemy_base (cast `/Game/Blueprints/Enemies/BP_EnemyBase` OtherActor))
  (bind _index (`self.CheckIndex` _asbp_enemy_base)
    (:`HasIndex`
      (`KismetArrayLibrary.Array_Remove` (`self.mEnemiesInRange`) _index))))

(fn `GetEnemyToFocus`
  (returns (Enemy :type "/Game/Blueprints/Enemies/BP_EnemyBase Object Reference"))
  (if (`KismetArrayLibrary.Array_IsNotEmpty` (`self.mEnemiesInRange`))
    (switch `/Game/Blueprints/Weapons/E_Focus` (`self.mFocus`)
      (:`NewEnumerator0`
        (for _array_element (`self.mEnemiesInRange`)
          (if (and (`KismetSystemLibrary.IsValid` _array_element) (not (`/Game/Blueprints/Enemies/BP_EnemyBase.dead` _array_element)))
            (`|ExecutionSequence`
              (:`then_0`
                (return _array_element))
              (:`then_1`
                (break)))))))
    (else
      (return null))))

(fn `GetFireRate`
  (params (`Fire Rate` :type "Float (double-precision)"))
  (returns (ReturnValue :type "Float (double-precision)"))
  (return (/ 1.0 `Fire Rate`)))

(fn `RotateToEnemy`
  (bind _mtarget (`self.mTarget`)
    (:`then`
      (bind (_x _y) (`KismetMathLibrary.BreakVector3f` (`KismetMathLibrary.BreakRotIntoAxes` (`KismetMathLibrary.FindLookAtRotation` (`SceneComponent.K2_GetComponentLocation` (`self.AxisX`)) (`self.K2_GetActorLocation` _mtarget)))))
      (`SceneComponent.K2_SetRelativeRotation` (`self.AxisX`) (`KismetMathLibrary.MakeRotationFromAxes` (`KismetMathLibrary.MakeVector` _x _y)) false false))
    (:`else`)))

(fn `UserConstructionScript`)