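; Base enemy Blueprint for a UFO that is moved by AI toward a waypoint while playing a procedural hover animation.
; On BeginPlay it spawns its default controller, then issues AIMoveTo to the first entry of MWaypoints, with no further waypoint logic.
; Each Tick, UFO_Anim yaws the EnemyUfoPurple component through Rotation and bobs its relative height with a sine of the accumulated phase UFOAnimP.
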(event `self.ReceiveBeginPlay`
  (`|ExecutionSequence`
    (:`then_0`
      (`self.SpawnDefaultController`))
    (:`then_1`
      (`|AIMoveTo` self (0.0 0.0 0.0) (`|GetArrayItem` (`self.mWaypoints`))))))

(event `self.ReceiveTick`
  (params (DeltaSeconds :type "Float (single-precision)"))
  (`self.UFO_Anim` DeltaSeconds 50.0 1.0 10.0))

(fn `UFO_Anim`
  (params (delta :type "Float (double-precision)") (rotationSpeed :type "Float (double-precision)") (floatingSpeed :type "Float (double-precision)") (floatingDistance :type "Float (double-precision)"))
  (bind _enemy_ufopurple (`self.enemy_ufoPurple`))
  (bind _returnvalue (+ (* delta floatingSpeed) (`self.UFO_AnimP`)))
  (bind (_relativerotation_roll _relativerotation_pitch _relativerotation_yaw) (`KismetMathLibrary.BreakRotator` (`SceneComponent.RelativeRotation` _enemy_ufopurple)))
  (`SceneComponent.K2_SetRelativeRotation` _enemy_ufopurple (`KismetMathLibrary.MakeRotator` 0.0 0.0 (+ _relativerotation_yaw (* delta rotationSpeed))) false false)
  (set `self.UFO_AnimP` _returnvalue)
  (`SceneComponent.K2_SetRelativeLocation` (`self.enemy_ufoPurple`) (`KismetMathLibrary.MakeVector` 0.0 0.0 (* (`KismetMathLibrary.Sin` _returnvalue) floatingDistance)) false false))

(fn `UserConstructionScript`)