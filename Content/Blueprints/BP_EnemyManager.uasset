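; BP_EnemyManager runs the enemy waves of a waypoint-based level and shows the win screen once all waves are cleared.
; After a short start delay, StartWave spawns each enemy class in the wave at the manager's transform, passing MWaypoints and pausing by that wave's cooldown.
; It then recurses to the next wave after a pause.
; When waves run out, a looping timer polls for remaining BP_EnemyBase actors and displays UW_Youve_Won when none remain.
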(event `self.ReceiveBeginPlay`
  (`KismetSystemLibrary.Delay` 5.0)
  (`self.StartWave` 0))

(event `StartWave`
  (params (Wave :type Integer))
  (bind (_spawncoldown _enemies) (break `/Game/Blueprints/Enemies/Waves/WaveStruct` (`|GetArrayItem` (`self.waves`) Wave)))
  (if (`KismetArrayLibrary.Array_IsValidIndex` (`self.waves`) Wave)
    (bind _output_get (set `self.EnemyIndex` 0))
    ;[0.32 0.9402 1] Create Enemy From Wave
    (if (`KismetArrayLibrary.Array_IsValidIndex` _enemies _output_get) :!label _label
      (`|SpawnActorFromClass` (`|GetArrayItem` _enemies _output_get) (`self.GetTransform`) "AlwaysSpawn" "MultiplyWithRoot" null (`self.mWaypoints`) null)
      (`/Engine/EditorBlueprintResources/StandardMacros.IncrementInt` (`self.EnemyIndex`)
        (:`  `
          (`KismetSystemLibrary.Delay` _spawncoldown)
          (goto _label)))
      (else
        ;[0.6017 1 0] Next Wave
        (`KismetSystemLibrary.Delay` 3.0)
        (`self.StartWave` (+ Wave 1))))
    (else
      ;[1 1 1] You Won
      (bind _returnvalue (`KismetSystemLibrary.K2_SetTimer` null "WinWidget" 5.0 true))
      (set `self.WinWIdgetTimer` _returnvalue))))

(fn `UserConstructionScript`)

(fn `WinWidget`
  (bind _outactors (`GameplayStatics.GetAllActorsOfClass` "/Game/Blueprints/Enemies/BP_EnemyBase.BP_EnemyBase_C"))
  (if (`KismetArrayLibrary.Array_IsEmpty` _outactors)
    (bind _returnvalue (`|CreateWidget` "/Game/HUD/UW_Youve_Won.UW_Youve_Won_C"))
    (`UserWidget.AddToViewport` _returnvalue 0)
    (`KismetSystemLibrary.K2_InvalidateTimerHandle` (`self.WinWIdgetTimer`))))